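; BP_JoyGiver is an old man interactable who periodically wishes for a joy gift that the player brings to him.
; After a random delay, he shows a thought widget and spawns the gift with smoke at a random location.
; Delivery consumes the held item, plays joy feedback, hands the player a spawned happy bubble and restarts the timer.
; Custom depth stencil highlights him for gift carriers, and he registers as an affected actor of the ColorCorrectionRegion.
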(event Custom|RespawnGift
  (Audio|PlaySound2D "/Game/Assets/SFX/OldMan/Tinking/SC_OldMandThinking.SC_OldMandThinking" 1.0 1.0 0.0 0 0)
  (Rendering|SetVisibility (Variables|Default|GetWW_Thoughts) true false)
  (bind _returnvalue (Niagara|SpawnSystematLocation "/Game/Assets/FX/NS_SmokeGift.NS_SmokeGift" (.OutItem (Utilities|Array|Random (Variables|Default|GetGiftSpawnLocation)))))
  (bind _returnvalue_2 (Game|SpawnActorfromClass "/Game/Assets/Blueprints/BP_JoyGift.BP_JoyGift_C" (Math|Transform|MakeTransform (Transformation|GetWorldLocation _returnvalue) "0, 0, 0" "1.000000,1.000000,1.000000") "Undefined" "MultiplyWithRoot" self 0))
  (Variables|Default|SetGiftRef _returnvalue_2))

(event Custom|StartPepe
  (Utilities|FlowControl|Delay (Math|Random|RandomFloatinRange (Variables|Default|GetMinRespawnTime) (Variables|Default|GetMaxRespawnTime)))
  (Audio|PlaySound2D "/Game/Assets/SFX/OldMan/Tinking/SC_OldMandThinking.SC_OldMandThinking" 1.0 1.0 0.0 0 0)
  (Rendering|SetVisibility (Variables|Default|GetWW_Thoughts) true false)
  (bind _returnvalue (Niagara|SpawnSystematLocation "/Game/Assets/FX/NS_SmokeGift.NS_SmokeGift" (.OutItem (Utilities|Array|Random (Variables|Default|GetGiftSpawnLocation)))))
  (bind _returnvalue_2 (Game|SpawnActorfromClass "/Game/Assets/Blueprints/BP_JoyGift.BP_JoyGift_C" (Math|Transform|MakeTransform (Transformation|GetWorldLocation _returnvalue) "0, 0, 0" "1.000000,1.000000,1.000000") "Undefined" "MultiplyWithRoot" self 0))
  (Variables|Default|SetGiftRef _returnvalue_2))

(event EventManageOutline
  (params (Active? :type Boolean))
  (bind _cylinder (Variables|Default|GetCylinder))
  (if (Utilities|Enum|Equal(Enum) (Variables|/Game/Assets/Blueprints/Player/BP_Player.BP_Player_C|GetItemHeld (Variables|/Game/Assets/Blueprints/Game/BP_Gamemode.BP_Gamemode_C|GetPlayerRef (CallFunction|GetGameModeRef))) "NewEnumerator5")
    (Rendering|SetCustomDepthStencilValue _cylinder (Math|Integer|SelectInt 2 1 Active?))
    (else
      (Rendering|SetCustomDepthStencilValue _cylinder 1))))

(event EventInteraction
  (params (PlayerRef :type BP%20Player%20Object%20Reference))
  (Variables|Default|GetGiftRef
    (:then
      (if (Utilities|Enum|Equal(Enum) (Variables|/Game/Assets/Blueprints/Player/BP_Player.BP_Player_C|GetItemHeld PlayerRef) "NewEnumerator5")
        (Audio|PlaySound2D "/Game/Assets/SFX/OldMan/Gratitude/SC_OldManGratitude.SC_OldManGratitude" 1.0 1.0 0.0 0 0)
        (Rendering|SetVisibility (Variables|Default|GetWW_Thoughts) false false)
        (Variables|/Game/Assets/Blueprints/Player/BP_Player.BP_Player_C|SetItemHeld PlayerRef "NewEnumerator0")
        (Actor|DestroyActor (Variables|/Game/Assets/Blueprints/Player/BP_Player.BP_Player_C|GetItemRef PlayerRef))
        (Variables|Default|SetGiftRef 0)
        (Development|PrintString "JOYYYYYYYYYY")
        (Components|Activation|Activate (Variables|Default|GetJoy) false)
        (bind _returnvalue (Game|SpawnActorfromClass "/Game/Assets/Blueprints/Bubble/BP_BubbleHappy.BP_BubbleHappy_C" (Math|Transform|MakeTransform "0, 0, 0" "0, 0, 0" "1.000000,1.000000,1.000000") "Undefined" "MultiplyWithRoot" 0 0))
        (Default|Interaction _returnvalue PlayerRef)
        (Utilities|Time|SetTimerbyEvent (delegate Custom|RespawnGift) (Math|Random|RandomFloatinRange (Variables|Default|GetMinRespawnTime) (Variables|Default|GetMaxRespawnTime)))
        (CallFunction|ManageOutline false)
        (Game|Feedback|PlayDynamicForceFeedback (Game|GetPlayerController 0) 0.2 0.1 true true true true)))
    (:else)))

(event EventBeginPlay
  (bind _returnvalue (Actor|GetActorOfClass "/Script/ColorCorrectRegions.ColorCorrectionRegion"))
  (Utilities|Set|Add (Variables|/Script/ColorCorrectRegions.ColorCorrectRegion|GetAffectedActors _returnvalue) (Utilities|ResolveSoftReference self)))

(fn ConstructionScript)