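; Game mode that opens the main menu and spawns player characters for solo or local co-op play.
; BeginPlay creates a stack widget, pushes the main menu onto it and keeps a reference.
; SpawnPlayer spawns and possesses Player 1 at the PlayerStart.
; With SelectCoop set, it also spawns Player 2 ahead of that point, creates a second local player to possess it, and tracks spawned players in PlayerArray.
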(event Custom|SpawnPlayer
  (bind _returnvalue (Actor|GetActorOfClass "/Script/Engine.PlayerStart"))
  (bind _returnvalue_2 (Game|SpawnActorfromClass "/Game/Assets/Blueprints/Player/BP_Player_1.BP_Player_1_C" (Math|Transform|MakeTransform (Transformation|GetActorLocation _returnvalue) "0, 0, 0" "1.000000,1.000000,1.000000") "AdjustIfPossibleButAlwaysSpawn" "MultiplyWithRoot" 0 0))
  (Pawn|Possess (CallFunction|GetPlayerControllerRef) _returnvalue_2)
  (Utilities|Array|Add (Variables|Default|GetPlayerArray) _returnvalue_2)
  (if (Variables|Default|GetbSelectCoop)
    (bind _returnvalue_3 (Game|SpawnActorfromClass "/Game/Assets/Blueprints/Player/BP_Player_2.BP_Player_2_C" (Math|Transform|MakeTransform (+ (Transformation|GetActorLocation _returnvalue) (* (Transformation|GetActorForwardVector _returnvalue) 3e+02)) "0, 0, 0" "1.000000,1.000000,1.000000") "AdjustIfPossibleButAlwaysSpawn" "MultiplyWithRoot" 0 0))
    (Class|GameplayStatics|CreatePlayer 1)
    (Pawn|Possess (Game|GetPlayerController 1) _returnvalue_3)
    (Utilities|Array|Add (Variables|Default|GetPlayerArray) _returnvalue_3)))

(event EventBeginPlay
  (bind _returnvalue (UserInterface|CreateWidget "/Game/Assets/UserWidget/Menu/WBP_StackWidget.WBP_StackWidget_C"))
  (Default|PushWidget _returnvalue "/Game/Assets/UserWidget/Menu/WBP_MainMenu.WBP_MainMenu_C")
  (Variables|Default|SetStackWidgetRef _returnvalue))

(fn ConstructionScript)