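; Player controller that handles the pause menu and creates the player HUD.
; The pause input toggles a stack widget, either creating one and pushing the pause menu onto it or tearing it down.
; Removal deactivates and detaches the stacked widget, clears the reference and unpauses the game.
; A separate function creates the HUD widget, stores it and adds it to the viewport.
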(event Custom|RemoveMenuPause
  (Class|CommonActivatableWidget|DeactivateWidget (Variables|/Game/Assets/UserWidget/Menu/WBP_StackWidget.WBP_StackWidget_C|GetWidgetRef (Variables|Default|GetWidgetStackRef)))
  (Widget|RemovefromParent (Variables|/Game/Assets/UserWidget/Menu/WBP_StackWidget.WBP_StackWidget_C|GetWidgetRef (Variables|Default|GetWidgetStackRef)))
  (Variables|Default|SetWidgetStackRef 0)
  (Game|SetGamePaused false))

(event Input|EnhancedActionEvents|EnhancedInputActionIA_Pause
  (params (ActionValue :type Boolean) (ElapsedSeconds :type Float%20%28double-precision%29) (TriggeredSeconds :type Float%20%28double-precision%29) (InputAction :type Input%20Action%20Object%20Reference :default "/Game/Assets/Inputs/Actions/IA_Pause.IA_Pause"))
  (:Started
    (Variables|Default|GetWidgetStackRef
      (:then
        (CallFunction|RemoveMenuPause))
      (:else
        (bind _returnvalue (UserInterface|CreateWidget "/Game/Assets/UserWidget/Menu/WBP_StackWidget.WBP_StackWidget_C"))
        (Default|PushWidget _returnvalue "/Game/Assets/UserWidget/Menu/WBP_PauseMenu.WBP_PauseMenu_C")
        (Variables|Default|SetWidgetStackRef _returnvalue)))))

(event EventBeginPlay)

(event EventTick
  (params (DeltaSeconds :type Float%20%28single-precision%29)))

(fn ConstructionScript)

(fn CreateWidgetPlayer
  (bind _returnvalue (UserInterface|CreateWidget "/Game/Assets/UserWidget/WBP_HUD.WBP_HUD_C"))
  (bind _output_get (Variables|Default|SetHUDRef _returnvalue))
  (UserInterface|Viewport|AddtoViewport _output_get 0))