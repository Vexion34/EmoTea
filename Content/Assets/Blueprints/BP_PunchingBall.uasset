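; Punching ball interactable that locks the player in place until they have hit it enough times.
; When the player's held-item state matches, the first interaction disables movement, and later ones drain HP with alternating left/right hit montages and controller rumble.
; At zero HP it resets, restores walking, spawns an angry bubble and forwards the interaction to it.
; A separate event toggles the cube's custom depth outline.
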(event EventManageOutline
  (params (Active? :type Boolean))
  (Rendering|SetRenderCustomDepth (Variables|Default|GetCube) Active?))

(event EventInteraction
  (params (PlayerRef :type BP%20Player%20Object%20Reference))
  (bind _mesh (Variables|/Script/Engine.Character|GetMesh PlayerRef))
  (if (Utilities|Enum|Equal(Enum) (Variables|/Game/Assets/Blueprints/Player/BP_Player.BP_Player_C|GetItemHeld PlayerRef) "NewEnumerator0")
    (if (not (Variables|Default|GetAttacked?))
      (Pawn|Components|CharacterMovement|SetMovementMode (Variables|/Script/Engine.Character|GetCharacterMovement PlayerRef) "MOVE_None" 0)
      (Variables|Default|SetAttacked? true)
      (else
        (bind _result (Math|Float|DecrementFloat (Variables|Default|GetHP))
          (:%20%20
            (Utilities|FlowControl|Sequence
              (:then_0
                (if (<= _result 0.0)
                  (Variables|Default|SetHP (Variables|Default|GetMaxHP))
                  (Variables|Default|SetAttacked? false)
                  (Pawn|Components|CharacterMovement|SetMovementMode (Variables|/Script/Engine.Character|GetCharacterMovement PlayerRef) "MOVE_Walking" 0)
                  (bind _returnvalue (Game|SpawnActorfromClass "/Game/Assets/Blueprints/Bubble/BP_BubbleAngry.BP_BubbleAngry_C" (Math|Transform|MakeTransform "0, 0, 0" "0, 0, 0" "1.000000,1.000000,1.000000") "Undefined" "MultiplyWithRoot" 0 0))
                  (Default|Interaction _returnvalue PlayerRef)))
              (:then_1
                (Utilities|FlowControl|FlipFlop
                  (:A
                    (Animation|Montage|PlayMontage _mesh "/Game/Assets/Chara/Anim/AM_HitL.AM_HitL"))
                  (:B
                    (Animation|Montage|PlayMontage _mesh "/Game/Assets/Chara/Anim/AM_HitR.AM_HitR"))))
              (:then_2
                (Game|Feedback|PlayDynamicForceFeedback (Game|GetPlayerController 0) 1.0 0.1 true true true true)))))))))

(fn ConstructionScript)