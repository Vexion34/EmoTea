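; BPFL_BubbleLibrary is a Blueprint function library of shortcut getters for the game's core objects.
; It returns the current game mode cast to BP_Gamemode and player controller 0 cast to BP_PlayerController.
; It also finds the BP_SpawnerManager in the world with a GetActorOfClass lookup, performed on each call without caching.
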(fn GetGameModeRef
  (bind _asbp_gamemode (Utilities|Casting|CastToBP_Gamemode (Game|GetGameMode (LocalVariables|Get__WorldContext))))
  (return _asbp_gamemode))

(fn GetSpawnManager
  (bind _returnvalue (Actor|GetActorOfClass (LocalVariables|Get__WorldContext) "/Game/Assets/Blueprints/Bubble/BP_SpawnerManager.BP_SpawnerManager_C"))
  (return _returnvalue))

(fn GetPlayerControllerRef
  (bind _asbp_player_controller (Utilities|Casting|CastToBP_PlayerController (Game|GetPlayerController (LocalVariables|Get__WorldContext))))
  (return _asbp_player_controller))