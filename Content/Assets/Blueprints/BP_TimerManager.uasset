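; BP_TimerManager is a match countdown that ticks down minutes and seconds and shows them on the player HUD.
; After a short delay on BeginPlay, it loads the max values and starts a looping one-second timer calling DecreaseTime.
; DecreaseTime rolls seconds into minutes and pushes the time to WBPTimer through BP_Gamemode's PlayerRef.
; Once minutes drop below zero, it clears the timer; the end-game step only prints a message.
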(event Custom|DecreaseTime
  (Development|PrintString "timer")
  (bind _result (Math|Float|DecrementFloat (Variables|Default|GetSeconds))
    (:%20%20
      (if (<= _result 0.0)
        (if (and (<= _result 0.0) (>= (Variables|Default|GetMinutes) 0.0))
          (Math|Float|DecrementFloat (Variables|Default|GetMinutes)
            (:%20%20
              (Variables|Default|SetSeconds 6e+01)
              (bind _asbp_gamemode (Utilities|Casting|CastToBP_Gamemode (Game|GetGameMode) :!label _label)
                (:then
                  (bind _playerref (Variables|/Game/Assets/Blueprints/Game/BP_Gamemode.BP_Gamemode_C|GetPlayerRef _asbp_gamemode)
                    (:then
                      (Default|SetCurrentTIme (Variables|/Game/Assets/UserWidget/WBP_HUD.WBP_HUD_C|GetWBP_Timer (Variables|/Game/Assets/Blueprints/Player/BP_Player.BP_Player_C|GetHUDRef _playerref)) (Variables|Default|GetMinutes) (Variables|Default|GetSeconds)))
                    (:else
                      (Development|PrintString "error" :!label _label_2))))
                (:CastFailed
                  (goto _label_2)))))
          (else
            (Utilities|Time|ClearandInvalidateTimerbyHandle (Variables|Default|GetTimerHandle))
            ;[1 1 1] EndGame
            (Development|PrintString "End")))
        (else
          (goto _label))))))

(event EventBeginPlay
  (Utilities|FlowControl|Delay 0.2)
  (Variables|Default|SetMinutes (Variables|Default|GetMaxMinutes))
  (Variables|Default|SetSeconds (Variables|Default|GetMaxSeconds))
  (bind _returnvalue (Utilities|Time|SetTimerbyEvent (delegate Custom|DecreaseTime) 1.0 true))
  (Variables|Default|SetTimerHandle _returnvalue)
  (bind _asbp_gamemode (Utilities|Casting|CastToBP_Gamemode (Game|GetGameMode)))
  (bind _playerref (Variables|/Game/Assets/Blueprints/Game/BP_Gamemode.BP_Gamemode_C|GetPlayerRef _asbp_gamemode)
    (:then
      (Default|SetCurrentTIme (Variables|/Game/Assets/UserWidget/WBP_HUD.WBP_HUD_C|GetWBP_Timer (Variables|/Game/Assets/Blueprints/Player/BP_Player.BP_Player_C|GetHUDRef _playerref)) (Variables|Default|GetMinutes) (Variables|Default|GetSeconds)))
    (:else)))

(fn ConstructionScript)