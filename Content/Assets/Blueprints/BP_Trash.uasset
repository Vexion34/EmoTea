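; BP_Trash is an interactable trash can that discards the player's held item, with sound, smoke and haptic feedback.
; Interaction clears and destroys the held item, removing bubble teas from the spawn manager's array.
; Certain item types also trigger respawns at BP_BowGiver or, after a random delay, BP_JoyGiver.
; It registers with a ColorCorrectionRegion on BeginPlay and toggles its outline through custom depth stencil.
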(event EventBeginPlay
  (bind _returnvalue (Actor|GetActorOfClass "/Script/ColorCorrectRegions.ColorCorrectionRegion"))
  (Utilities|Set|Add (Variables|/Script/ColorCorrectRegions.ColorCorrectRegion|GetAffectedActors _returnvalue) (Utilities|ResolveSoftReference self)))

(event EventManageOutline
  (params (Active? :type Boolean))
  (Rendering|SetCustomDepthStencilValue (Variables|Default|GetCube) (Math|Integer|SelectInt 2 1 Active?)))

(event EventInteraction
  (params (PlayerRef :type BP%20Player%20Object%20Reference))
  (if (Utilities|Enum|NotEqual(Enum) (Variables|/Game/Assets/Blueprints/Player/BP_Player.BP_Player_C|GetItemHeld PlayerRef) "NewEnumerator0")
    (Audio|PlaySound2D "/Game/Assets/SFX/SFX_ThrowInTrash.SFX_ThrowInTrash" 1.0 1.0 0.0 0 0)
    (Utilities|FlowControl|Sequence
      (:then_0
        (Utilities|FlowControl|Sequence
          (:then_0
            (if (Utilities|Enum|Equal(Enum) (Variables|/Game/Assets/Blueprints/Player/BP_Player.BP_Player_C|GetItemHeld PlayerRef) "NewEnumerator1")
              (bind _returnvalue (Actor|GetActorOfClass "/Game/Assets/Blueprints/BP_BowGiver.BP_BowGiver_C"))
              (Default|RespawnBow _returnvalue)))
          (:then_1
            (if (Utilities|Enum|Equal(Enum) (Variables|/Game/Assets/Blueprints/Player/BP_Player.BP_Player_C|GetItemHeld PlayerRef) "NewEnumerator5")
              (bind _returnvalue_2 (Actor|GetActorOfClass "/Game/Assets/Blueprints/BP_JoyGiver.BP_JoyGiver_C"))
              (Utilities|FlowControl|Delay (Math|Random|RandomFloatinRange 2.0 5.0))
              (Default|RespawnGift _returnvalue_2)))))
      (:then_1
        (Default|BreakEffect PlayerRef)
        (Variables|/Game/Assets/Blueprints/Player/BP_Player.BP_Player_C|SetItemHeld PlayerRef "NewEnumerator0")
        (Niagara|SpawnSystematLocation "/Game/Assets/FX/NS_SmokeTrash.NS_SmokeTrash" (Transformation|GetWorldLocation (Variables|/Game/Assets/Blueprints/Player/BP_Player.BP_Player_C|GetGrabbingScene PlayerRef)))
        (Default|DeactivateNiagaraBubble PlayerRef)
        (bind _itemref (Variables|/Game/Assets/Blueprints/Player/BP_Player.BP_Player_C|GetItemRef PlayerRef)
          (:then
            (bind _asbp_bubble_tea_2 (Utilities|Casting|CastToBP_BubbleTea2 _itemref)
              (:then
                (Utilities|Array|RemoveItem (Variables|/Game/Assets/Blueprints/Bubble/BP_SpawnerManager.BP_SpawnerManager_C|GetBubbleTeaArray (CallFunction|GetSpawnManager)) _asbp_bubble_tea_2)
                (Actor|DestroyActor _asbp_bubble_tea_2))
              (:CastFailed
                (Actor|DestroyActor _itemref)))
            (Game|Feedback|PlayDynamicForceFeedback (Game|GetPlayerController 0) 0.4 0.1 true true true true))
          (:else))))))

(fn ConstructionScript)