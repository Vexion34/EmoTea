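; BP_LoveInteract is an interactable pickup, apparently a bow, that the player can take and that can respawn elsewhere.
; Interaction checks the player's held-item enum, switches it to the next entry, plays brief controller rumble and hides the actor instead of destroying it.
; RespawnBow moves it to a random respawn location and unhides it.
; ManageOutline toggles custom depth on the Cube for highlighting.
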(event Custom|RespawnBow
  (Transformation|SetActorLocation (.OutItem (Utilities|Array|Random (Variables|Default|GetRespawnLocation))) false false)
  (Rendering|SetActorHiddenInGame false))

(event EventManageOutline
  (params (Active? :type Boolean))
  (Rendering|SetRenderCustomDepth (Variables|Default|GetCube) Active?))

(event EventInteraction
  (params (PlayerRef :type BP%20Player%20Object%20Reference))
  (if (Utilities|Enum|Equal(Enum) (Variables|/Game/Assets/Blueprints/Player/BP_Player.BP_Player_C|GetItemHeld PlayerRef) "NewEnumerator0")
    (Variables|/Game/Assets/Blueprints/Player/BP_Player.BP_Player_C|SetItemHeld PlayerRef "NewEnumerator1")
    (Game|Feedback|PlayDynamicForceFeedback (Game|GetPlayerController 0) 0.2 0.1 true true true true)
    (Rendering|SetActorHiddenInGame true)))

(fn ConstructionScript)