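; BP_Table is an interactable table where the player sets down a held item.
; On interaction, a sphere trace above the table looks for a Destructible-type object and forwards the interaction to it if found.
; Otherwise, a held item is detached, moved to DroppedLocation and cleared from the player, with a pickup sound.
; One item type, apparently the bow, instead relocates and unhides the level's BP_BowGiver.
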(event EventInteraction
  (params (PlayerRef :type BP%20Player%20Object%20Reference))
  (bind _returnvalue (Transformation|GetActorLocation))
  (bind (_outhit _returnvalue_2) (Collision|SphereTraceForObjects _returnvalue (+ _returnvalue "0.000000,0.000000,100.000000") 25.0 (Utilities|Array|MakeArray "ObjectTypeQuery6") false 0 "ForDuration"))
  (if _returnvalue_2
    (Class|BPIInteract|Interaction(Message) (.HitActor (Collision|BreakHitResult _outhit)) PlayerRef)
    (elif (Utilities|Enum|NotEqual(Enum) (Variables|/Game/Assets/Blueprints/Player/BP_Player.BP_Player_C|GetItemHeld PlayerRef) "NewEnumerator0")
      (Audio|PlaySound2D "/Game/Assets/SFX/PickUp/SC_PickupItem.SC_PickupItem" 1.0 1.0 0.0 0 0)
      (if (Utilities|Enum|NotEqual(Enum) (Variables|/Game/Assets/Blueprints/Player/BP_Player.BP_Player_C|GetItemHeld PlayerRef) "NewEnumerator1")
        (Transformation|DetachFromActor (Variables|/Game/Assets/Blueprints/Player/BP_Player.BP_Player_C|GetItemRef PlayerRef) "KeepWorld" "KeepWorld" "KeepWorld")
        (Transformation|SetActorLocation (Variables|/Game/Assets/Blueprints/Player/BP_Player.BP_Player_C|GetItemRef PlayerRef) (Transformation|GetWorldLocation (Variables|Default|GetDroppedLocation)) false false)
        (Class|BPIInteract|ManageCollisions(Message) (Variables|/Game/Assets/Blueprints/Player/BP_Player.BP_Player_C|GetItemRef PlayerRef) false)
        (Variables|/Game/Assets/Blueprints/Player/BP_Player.BP_Player_C|SetItemRef PlayerRef 0)
        (Variables|/Game/Assets/Blueprints/Player/BP_Player.BP_Player_C|SetItemHeld PlayerRef "NewEnumerator0")
        (else
          (bind _returnvalue_3 (Actor|GetActorOfClass "/Game/Assets/Blueprints/BP_BowGiver.BP_BowGiver_C"))
          (Transformation|SetActorLocation _returnvalue_3 (Transformation|GetWorldLocation (Variables|Default|GetDroppedLocation)) false false)
          (Rendering|SetActorHiddenInGame _returnvalue_3 false)
          (Variables|/Game/Assets/Blueprints/Player/BP_Player.BP_Player_C|SetItemHeld PlayerRef "NewEnumerator0"))))))

(fn ConstructionScript)