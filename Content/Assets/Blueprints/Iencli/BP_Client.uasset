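; Customer (client) actor that generates bubble tea orders and receives the drinks players deliver.
; A looping timer picks random DataRecette rows and adds WBP_Recette widgets to the HUD, up to five at once.
; Interaction compares the held BP_BubbleTea2's bubble types against each order, destroys the drink regardless, and removes the matched order widget.
; Tick and the matching loop print debug strings.
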(event Custom|Test
  (if (< (Utilities|Array|LastIndex (Variables|Default|GetRecetteWidgetArray)) 4)
    (bind _outrownames (DataTable|GetDataTableRowNames (Variables|Default|GetDataRecette)))
    (bind _output_get (Variables|Default|SetRecetteName (.OutItem (Utilities|Array|Random _outrownames))))
    (bind _returnvalue (Utilities|GetDataTableRow (Variables|Default|GetDataRecette) _output_get)
      (:then
        (bind _returnvalue_2 (UserInterface|CreateWidget "/Game/Assets/UserWidget/WBP_Recette.WBP_Recette_C" 0 (.IconBubbleRequired (Utilities|Struct|BreakS_Recette _returnvalue)) (.BubbleRequired (Utilities|Struct|BreakS_Recette _returnvalue))))
        (Utilities|Array|Add (Variables|Default|GetRecetteWidgetArray) _returnvalue_2)
        (Class|HorizontalBox|AddChildtoHorizontalBox (Variables|/Game/Assets/UserWidget/WBP_HUD.WBP_HUD_C|GetHb_Recette (Variables|/Game/Assets/Blueprints/Game/BP_PlayerController.BP_PlayerController_C|GetHUDRef (CallFunction|GetPlayerControllerRef))) _returnvalue_2)
        (Class|Image|SetBrush (Variables|/Game/Assets/UserWidget/WBP_Recette.WBP_Recette_C|GetBubbleTeaIcon _returnvalue_2) (Utilities|Struct|MakeSlateBrush "Image" "NoTile" "NoMirror" (Utilities|Struct|MakeDeprecateSlateVector2D 6e+01 6e+01) "(Left=0.000000,Top=0.000000,Right=0.000000,Bottom=0.000000)" "(SpecifiedColor=(R=1.000000,G=1.000000,B=1.000000,A=1.000000),ColorUseRule=UseColor_Specified)" "(CornerRadii=(X=0.000000,Y=0.000000,Z=0.000000,W=0.000000),Color=(SpecifiedColor=(R=0.000000,G=0.000000,B=0.000000,A=0.000000),ColorUseRule=UseColor_Specified),Width=0.000000,RoundingType=HalfHeightRadius,bUseBrushTransparency=False)" (.SpriteBubbleTea (Utilities|Struct|BreakS_Recette _returnvalue))))
        (Default|SetUpIconRequired _returnvalue_2)))))

(event EventBeginPlay
  (Utilities|Time|SetTimerbyEvent (delegate Custom|Test) (Math|Random|RandomFloatinRange 5.0 8.0) true false -4.0))

(event Collision|EventActorBeginOverlap
  (params (OtherActor :type Actor%20Object%20Reference)))

(event EventTick
  (params (DeltaSeconds :type Float%20%28single-precision%29))
  (Development|PrintString (Utilities|GetDisplayName (Variables|Default|GetWidgetElement)) true true "(R=0.863621,G=1.000000,B=0.096568,A=1.000000)" 0.0))

(event EventInteraction
  (params (PlayerRef :type BP%20Player%20Object%20Reference))
  (bind _asbp_bubble_tea_2 (Utilities|Casting|CastToBP_BubbleTea2 (Variables|/Game/Assets/Blueprints/Player/BP_Player.BP_Player_C|GetItemRef PlayerRef)))
  (bind _array_element (Utilities|Array|ForEachLoopwithBreak (Variables|Default|GetRecetteWidgetArray) :!label _label)
    (:LoopBody
      (if (<= (Utilities|Array|LastIndex (Variables|/Game/Assets/Blueprints/Bubble/BP_BubbleTea2.BP_BubbleTea2_C|GetArrayTypeBubble _asbp_bubble_tea_2)) (Utilities|Array|LastIndex (Variables|/Game/Assets/UserWidget/WBP_Recette.WBP_Recette_C|GetRecetteTypeArray _array_element)))
        (bind _array_element_2 (Utilities|Array|ForEachLoopwithBreak (Variables|/Game/Assets/UserWidget/WBP_Recette.WBP_Recette_C|GetRecetteTypeArray _array_element))
          (:LoopBody
            (if (!= (Utilities|Array|FindItem (Variables|/Game/Assets/Blueprints/Bubble/BP_BubbleTea2.BP_BubbleTea2_C|GetArrayTypeBubble _asbp_bubble_tea_2) _array_element_2) -1)
              (bind _result (Math|Integer|IncrementInt (Variables|Default|Getteste))
                (:%20%20
                  (Development|PrintString (Utilities|String|ToString(Integer) _result))
                  (if (== _result (+ (Utilities|Array|LastIndex (Variables|/Game/Assets/UserWidget/WBP_Recette.WBP_Recette_C|GetRecetteTypeArray _array_element)) 1))
                    (Variables|Default|SetWidgetElement _array_element)
                    (goto _label Break))))))
          (:Completed
            (Variables|Default|Setteste 0)))))
    (:Completed
      (bind _asbp_bubble_tea_2_2 (Utilities|Casting|CastToBP_BubbleTea2 (Variables|/Game/Assets/Blueprints/Player/BP_Player.BP_Player_C|GetItemRef PlayerRef)))
      (Utilities|Array|Clear (Variables|/Game/Assets/Blueprints/Bubble/BP_BubbleTea2.BP_BubbleTea2_C|GetArrayTypeBubble _asbp_bubble_tea_2_2))
      (Utilities|Array|RemoveItem (Variables|/Game/Assets/Blueprints/Bubble/BP_SpawnerManager.BP_SpawnerManager_C|GetBubbleTeaArray (CallFunction|GetSpawnManager)) _asbp_bubble_tea_2_2)
      (Actor|DestroyActor _asbp_bubble_tea_2_2)
      (bind _widgetelement (Variables|Default|GetWidgetElement)
        (:then
          (Widget|RemovefromParent _widgetelement)
          (Utilities|Array|RemoveItem (Variables|Default|GetRecetteWidgetArray) _widgetelement))
        (:else)))))

(fn ConstructionScript)