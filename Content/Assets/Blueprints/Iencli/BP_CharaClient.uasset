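; Client character that walks through a queue using AI MoveTo and shares its state through the spawn manager's client array.
; On arrival it takes the given yaw and has the spawn manager spawn a recipe (SpawnRecette).
; When leaving, it immediately removes itself from the queue, sends the new front client to the start spot and shifts each other client to its predecessor's position.
; It destroys itself on reaching the exit.
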(event Custom|MoveToLocation
  (params (Destination :type Vector) (Rotation :type Rotator))
  (AI|AIMoveTo self Destination 0 5.0 false
    (:OnSuccess
      (Transformation|SetActorRotation (Math|Rotator|MakeRotator 0.0 0.0 (.Yaw (Math|Rotator|BreakRotator Rotation))))
      (Default|SpawnRecette (CallFunction|GetSpawnManager)))))

(event Custom|MoveToLeaveLocation
  (params (DestinationEnd :type Vector) (DestinationStart :type Vector))
  (bind _managerref (CallFunction|GetSpawnManager))
  (bind _clientarray (Variables|/Game/Assets/Blueprints/Bubble/BP_SpawnerManager.BP_SpawnerManager_C|GetClientArray _managerref))
  (AI|AIMoveTo self DestinationEnd 0 5.0 false
    (:then
      (Math|Integer|DecrementInt (Variables|/Game/Assets/Blueprints/Bubble/BP_SpawnerManager.BP_SpawnerManager_C|GetIndexClient _managerref)
        (:%20%20
          (Utilities|Array|RemoveItem _clientarray self)
          (if (Utilities|Array|IsValidIndex _clientarray)
            (CallFunction|MovetoLocation (Utilities|Array|Get(acopy) _clientarray) DestinationStart (Transformation|GetActorRotation (Variables|/Game/Assets/Blueprints/Bubble/BP_SpawnerManager.BP_SpawnerManager_C|GetClientDestination _managerref)))
            (CallFunction|MoveAllClient)))))
    (:OnSuccess
      (Actor|DestroyActor))))

(event Custom|MoveAllClient
  (bind _managerref (CallFunction|GetSpawnManager))
  (bind _clientarray (Variables|/Game/Assets/Blueprints/Bubble/BP_SpawnerManager.BP_SpawnerManager_C|GetClientArray _managerref))
  (for (_array_element _array_index) _clientarray
    (if (!= _array_index 0)
      (CallFunction|MovetoLocation _array_element (Transformation|GetActorLocation (Utilities|Array|Get(acopy) _clientarray (- _array_index 1))) "0, 0, 0"))))

(event EventBeginPlay)

(event Collision|EventActorBeginOverlap
  (params (OtherActor :type Actor%20Object%20Reference)))

(event EventTick
  (params (DeltaSeconds :type Float%20%28single-precision%29)))

(fn ConstructionScript)