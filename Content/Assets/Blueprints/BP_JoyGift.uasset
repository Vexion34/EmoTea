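; BP_JoyGift is a gift pickup that the player takes in hand by interacting with it.
; Its Interaction event checks the player's ItemHeld state and, on a match, switches it to another enum value and snaps the gift to the GrabbingScene component, keeping world scale.
; It then disables collision on its Cube and plays a brief force-feedback pulse on the first player controller.
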(event EventInteraction
  (params (PlayerRef :type BP%20Player%20Object%20Reference))
  (if (Utilities|Enum|Equal(Enum) (Variables|/Game/Assets/Blueprints/Player/BP_Player.BP_Player_C|GetItemHeld PlayerRef) "NewEnumerator0")
    (Variables|/Game/Assets/Blueprints/Player/BP_Player.BP_Player_C|SetItemHeld PlayerRef "NewEnumerator5")
    (Transformation|AttachComponentToComponent self (Variables|/Game/Assets/Blueprints/Player/BP_Player.BP_Player_C|GetGrabbingScene PlayerRef) "None" "SnapToTarget" "SnapToTarget" "KeepWorld" true)
    (Collision|SetCollisionEnabled (Variables|Default|GetCube) "NoCollision")
    (Game|Feedback|PlayDynamicForceFeedback (Game|GetPlayerController 0) 0.2 0.1 true true true true)))

(fn ConstructionScript)