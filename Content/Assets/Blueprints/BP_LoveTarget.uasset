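; BP_LoveTarget is a target actor that responds when a BP_LoveProjectile overlaps its Cube.
; A hit spawns a heart explosion effect, destroys the projectile and resets the player's held item through BP_Gamemode's PlayerRef.
; It then spawns a BP_BubbleLove at SpawnLocation, plays brief controller force feedback and tells the level's BP_LoveInteract to respawn the bow.
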(event OnComponentBeginOverlap(Cube)
  (params (OverlappedComponent :type Primitive%20Component%20Object%20Reference) (OtherActor :type Actor%20Object%20Reference) (OtherComp :type Primitive%20Component%20Object%20Reference) (OtherBodyIndex :type Integer) (bFromSweep :type Boolean) (SweepResult :type Hit%20Result%20Structure%20%28by%20ref%29))
  (bind _asbp_love_projectile (Utilities|Casting|CastToBP_LoveProjectile OtherActor))
  (Niagara|SpawnSystematLocation "/Game/Assets/FX/NS_HeartExplosion.NS_HeartExplosion" (Transformation|GetActorLocation _asbp_love_projectile))
  (Actor|DestroyActor _asbp_love_projectile)
  (bind _asbp_gamemode (Utilities|Casting|CastToBP_Gamemode (Game|GetGameMode)))
  (Variables|/Game/Assets/Blueprints/Player/BP_Player.BP_Player_C|SetItemHeld (Variables|/Game/Assets/Blueprints/Game/BP_Gamemode.BP_Gamemode_C|GetPlayerRef _asbp_gamemode) "NewEnumerator0")
  (Game|SpawnActorfromClass "/Game/Assets/Blueprints/Bubble/BP_BubbleLove.BP_BubbleLove_C" (Math|Transform|MakeTransform (Transformation|GetWorldLocation (Variables|Default|GetSpawnLocation)) "0, 0, 0" "1.000000,1.000000,1.000000") "Undefined" "MultiplyWithRoot" 0 0)
  (Game|Feedback|PlayDynamicForceFeedback (Game|GetPlayerController 0) 0.5 0.1 true true true true)
  (bind _returnvalue (Actor|GetActorOfClass "/Game/Assets/Blueprints/BP_LoveInteract.BP_LoveInteract_C"))
  (Default|RespawnBow _returnvalue))

(fn ConstructionScript)