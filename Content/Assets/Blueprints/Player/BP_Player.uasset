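; Player character Blueprint that aims at the mouse cursor, dashes, interacts with objects and shoots love projectiles from a bow.
; Tick traces under the moved cursor to set yaw, and dash launches the character forward with Niagara effects and a cooldown.
; Interact sphere-traces Destructible objects and messages hits; in one held-item state, holding it stops movement and release fires at FireRate if nothing is hit.
; Sphere overlaps toggle outlines on nearby actors.
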(event OnComponentBeginOverlap(Sphere)
  (params (OverlappedComponent :type Primitive%20Component%20Object%20Reference) (OtherActor :type Actor%20Object%20Reference) (OtherComp :type Primitive%20Component%20Object%20Reference) (OtherBodyIndex :type Integer) (bFromSweep :type Boolean) (SweepResult :type Hit%20Result%20Structure%20%28by%20ref%29))
  (Class|BPIInteract|ManageOutline(Message) OtherActor true))

(event OnComponentEndOverlap(Sphere)
  (params (OverlappedComponent :type Primitive%20Component%20Object%20Reference) (OtherActor :type Actor%20Object%20Reference) (OtherComp :type Primitive%20Component%20Object%20Reference) (OtherBodyIndex :type Integer))
  (Class|BPIInteract|ManageOutline(Message) OtherActor false))

(event Input|EnhancedActionEvents|EnhancedInputActionIA_Move
  (params (ActionValue :type Vector%202D%20Structure) (ElapsedSeconds :type Float%20%28double-precision%29) (TriggeredSeconds :type Float%20%28double-precision%29) (InputAction :type Input%20Action%20Object%20Reference :default "/Game/Assets/Inputs/Actions/IA_Move.IA_Move"))
  (bind (_x _y) (Math|Vector2D|BreakVector2D ActionValue))
  (if (Utilities|Enum|Equal(Enum) (Variables|Default|GetItemHeld) "NewEnumerator1")
    (Transformation|SetActorRotation (Math|Interpolation|RInterpTo (Transformation|GetActorRotation) (Math|Conversions|RotationFromXVector (Math|Vector|MakeVector _y _x 0.0)) (Utilities|Time|GetWorldDeltaSeconds) 1e+01))
    (Development|PrintString "rotating" true true "(R=0.000000,G=0.660000,B=1.000000,A=1.000000)" 0.0)))

(event Input|EnhancedActionEvents|EnhancedInputActionIA_Dash
  (params (ActionValue :type Boolean) (ElapsedSeconds :type Float%20%28double-precision%29) (TriggeredSeconds :type Float%20%28double-precision%29) (InputAction :type Input%20Action%20Object%20Reference :default "/Game/Assets/Inputs/Actions/IA_Dash.IA_Dash"))
  (bind _returnvalue (Transformation|GetVelocity))
  (bind (_x _y) (Math|Vector|BreakVector _returnvalue))
  (:Started
    (if (Math|Boolean|ANDBoolean (Utilities|Enum|Equal(Enum) (Variables|/Script/Engine.CharacterMovementComponent|GetMovementMode (Variables|Character|GetCharacterMovement)) "MOVE_Walking") (Variables|Default|GetCanDash?) (or (!= _x 0.0) (!= _y 0.0)))
      (Variables|Default|SetCanDash? false)
      (Character|LaunchCharacter (* (Transformation|GetActorForwardVector) (Variables|Default|GetDashPower)) false false)
      (Development|PrintString "Dash" true true "(R=1.000000,G=0.000000,B=0.193203,A=1.000000)")
      (Niagara|SpawnSystematLocation "/Game/Assets/FX/NS_Dash.NS_Dash" (Transformation|GetActorLocation) (Transformation|GetActorRotation))
      (Utilities|FlowControl|Delay 2.0)
      (Variables|Default|SetCanDash? true))))

(event Input|EnhancedActionEvents|EnhancedInputActionIA_Interact
  (params (ActionValue :type Boolean) (ElapsedSeconds :type Float%20%28double-precision%29) (TriggeredSeconds :type Float%20%28double-precision%29) (InputAction :type Input%20Action%20Object%20Reference :default "/Game/Assets/Inputs/Actions/IA_Interact.IA_Interact"))
  (:Started
    (if (Utilities|Enum|Equal(Enum) (Variables|Default|GetItemHeld) "NewEnumerator1")
      (Pawn|Components|CharacterMovement|SetMovementMode (Variables|Character|GetCharacterMovement) "MOVE_None" 0)))
  (:Completed
    (if (Utilities|Enum|NotEqual(Enum) (Variables|Default|GetItemHeld) "NewEnumerator1")
      (CallFunction|Interaction)
      (else
        (Pawn|Components|CharacterMovement|SetMovementMode (Variables|Character|GetCharacterMovement) "MOVE_Walking" 0)
        (if (Variables|Default|GetCanShoot?)
          (bind _hashit (CallFunction|Interaction))
          (if (not _hashit)
            (CallFunction|ShootBow)
            (Utilities|FlowControl|Delay (/ (Variables|Default|GetFireRate) 1.0))
            (Variables|Default|SetCanShoot? true)))))))

(event EventBeginPlay
  (Input|AddMappingContext (PlayerController|LocalPlayerSubsystems|GetEnhancedInputLocalPlayerSubsystem (Game|GetPlayerController 0)) "/Game/Assets/Inputs/IMC_Default.IMC_Default" 0 "(bIgnoreAllPressedKeysUntilRelease=True,bForceImmediately=False,bNotifyUserSettings=False)")
  (Development|PrintString "Hello")
  (Variables|Default|SetBaseMaxWalkSpeed (Variables|/Script/Engine.CharacterMovementComponent|GetMaxWalkSpeed (Variables|Character|GetCharacterMovement)))
  (Variables|/Game/Assets/Blueprints/Game/BP_Gamemode.BP_Gamemode_C|SetPlayerRef (CallFunction|GetGameModeRef) self)
  (Class|PlayerController|SetAudioListenerOverride (CallFunction|GetPlayerControllerRef) (Variables|Character|GetMesh) "0, 0, 0" "0, 0, 0"))

(event EventTick
  (params (DeltaSeconds :type Float%20%28single-precision%29))
  (bind _pcref (CallFunction|GetPlayerControllerRef))
  (bind _returnvalue (Transformation|GetActorRotation))
  (bind _worldlocation (Game|Player|ConvertMouseLocationToWorldSpace _pcref))
  (bind (_worldlocation_2 _worlddirection) (Game|Player|ConvertMouseLocationToWorldSpace _pcref))
  (if (Utilities|Operators|NotEqual(!=) (Variables|Default|GetWorld%20Location) _worldlocation 0.0)
    (Variables|Default|SetWorld%20Location _worldlocation)
    (bind (_outhit _returnvalue_2) (Collision|LineTraceByChannel _worldlocation_2 (+ (* _worlddirection 8e+03) _worldlocation_2) "TraceTypeQuery1" false 0 "None"))
    (if _returnvalue_2
      (Transformation|SetActorRotation (Math|Rotator|MakeRotator (.roll _returnvalue) (.pitch _returnvalue) (.yaw (Math|Rotator|FindLookatRotation (Transformation|GetActorLocation) (.Location (Collision|BreakHitResult _outhit)))))))))

(fn ConstructionScript)

(fn Interaction
  (bind _returnvalue (Transformation|GetActorLocation))
  (Development|PrintString "Interact")
  (bind (_outhit _returnvalue_2) (Collision|SphereTraceForObjects _returnvalue (+ _returnvalue (* (Transformation|GetActorForwardVector) (Variables|Default|GetRange))) 5e+01 (Utilities|Array|MakeArray "ObjectTypeQuery6") false 0 "ForDuration"))
  (if _returnvalue_2
    (Class|BPIInteract|Interaction(Message) (.HitActor (Collision|BreakHitResult _outhit)) self)
    (return _returnvalue_2 (.HitActor (Collision|BreakHitResult _outhit)))
    (else
      (return _returnvalue_2 0))))

(fn ShootBow
  (bind _shootout (Variables|Default|GetShootOut))
  (bind _returnvalue (Transformation|GetWorldTransform _shootout))
  (bind (_location _rotation) (Math|Transform|BreakTransform _returnvalue))
  (Variables|Default|SetCanShoot? false)
  (Game|SpawnActorfromClass "/Game/Assets/Blueprints/BP_LoveProjectile.BP_LoveProjectile_C" (Math|Transform|MakeTransform _location _rotation) "Undefined" "MultiplyWithRoot" 0 0)
  (Pawn|Components|CharacterMovement|SetMovementMode (Variables|Character|GetCharacterMovement) "MOVE_Walking" 0))