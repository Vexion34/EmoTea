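; Manager that spawns bubble teas and queuing clients with recipe orders, paced by difficulty.
; A looping timer, with its random interval rolled once, fills random spawn points up to a cap, line-tracing for static ground and retrying on a miss.
; Each client spawn adds a HUD recipe from a data table, using difficulty-weighted rejection sampling by required-bubble count.
; Each order schedules the next client while recipe slots remain; nothing here triggers the first.
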(event Custom|LaunchSpawnerRecetteTimer
  (if (< (Utilities|Array|LastIndex (Variables|Default|GetRecetteWidgetArray)) 4)
    (CallFunction|SpawnClient)))

(event Custom|SpawnerTimer
  (Utilities|Time|SetTimerbyEvent (delegate Custom|SpawnBubbleTea) (Math|Random|RandomFloatinRange (Variables|Default|GetBubbleTeaSpawnRateMin) (Variables|Default|GetBubbleTeaSpawnRateMax)) true))

(event Custom|FirstBubbleTeaSpawn
  (for _index (range 0 (- (Variables|Default|GetNumberOfFirstBubbleTea) 1))
    (CallFunction|SpawnBubbleTea))
  (CallFunction|SpawnerTimer))

(event Custom|SpawnBubbleTea
  (if (< (Utilities|Array|LastIndex (Variables|Default|GetBubbleTeaArray)) (- (Variables|Default|GetMaxBubble) 1))
    (bind _output_get (Variables|Default|SetSpawnPoint (.OutItem (Utilities|Array|Random (Variables|Default|GetSpawnablePoint)))))
    (bind (_outhit _returnvalue) (Collision|LineTraceForObjects (+ (Transformation|GetActorLocation _output_get) "0.000000,0.000000,500.000000") (- (Transformation|GetActorLocation _output_get) "0.000000,0.000000,1000.000000") (Utilities|Array|MakeArray "ObjectTypeQuery1") false 0 "ForDuration"))
    (if _returnvalue
      (Variables|Default|SetSpawnTestCount 0)
      (bind _returnvalue_2 (Game|SpawnActorfromClass "/Game/Assets/Blueprints/Bubble/BP_BubbleTea2.BP_BubbleTea2_C" (Math|Transform|MakeTransform (Transformation|GetActorLocation (Variables|Default|GetSpawnPoint)) (Transformation|GetActorRotation (Variables|Default|GetSpawnPoint)) "1.000000,1.000000,1.000000") "AlwaysSpawn" "MultiplyWithRoot" 0 0))
      (Utilities|Array|Add (Variables|Default|GetBubbleTeaArray) _returnvalue_2)
      (else
        (bind _result (Math|Integer|IncrementInt (Variables|Default|GetSpawnTestCount))
          (:%20%20
            (if (not (== _result (Utilities|Array|LastIndex (Variables|Default|GetSpawnablePoint))))
              (CallFunction|ChooseOtherSpawnPoint))))))))

(event Custom|ChooseOtherSpawnPoint
  (bind _output_get (Variables|Default|SetSpawnPoint (.OutItem (Utilities|Array|Random (Variables|Default|GetSpawnablePoint)))))
  (bind (_outhit _returnvalue) (Collision|LineTraceForObjects (+ (Transformation|GetActorLocation _output_get) "0.000000,0.000000,500.000000") (- (Transformation|GetActorLocation _output_get) "0.000000,0.000000,1000.000000") (Utilities|Array|MakeArray "ObjectTypeQuery1") false 0 "ForDuration"))
  (if _returnvalue
    (Variables|Default|SetSpawnTestCount 0)
    (bind _returnvalue_2 (Game|SpawnActorfromClass "/Game/Assets/Blueprints/Bubble/BP_BubbleTea2.BP_BubbleTea2_C" (Math|Transform|MakeTransform (Transformation|GetActorLocation (Variables|Default|GetSpawnPoint)) (Transformation|GetActorRotation (Variables|Default|GetSpawnPoint)) "1.000000,1.000000,1.000000") "AlwaysSpawn" "MultiplyWithRoot" 0 0))
    (Utilities|Array|Add (Variables|Default|GetBubbleTeaArray) _returnvalue_2)
    (else
      (bind _result (Math|Integer|IncrementInt (Variables|Default|GetSpawnTestCount))
        (:%20%20
          (if (not (== _result (Utilities|Array|LastIndex (Variables|Default|GetSpawnablePoint))))
            (CallFunction|ChooseOtherSpawnPoint)))))))

(event Custom|SpawnerRecette
  (Utilities|Time|SetTimerbyEvent (delegate Custom|LaunchSpawnerRecetteTimer) (Math|Random|RandomFloatinRange (Variables|Default|GetSpawnRecetteMinRate) (Variables|Default|GetSpawnRecetteMaxRate))))

(event Custom|SpawnClient
  (bind _clientdestination (Variables|Default|GetClientDestination))
  (bind _clientarray (Variables|Default|GetClientArray))
  (Utilities|FlowControl|Sequence
    (:then_0
      (bind _returnvalue (Game|SpawnActorfromClass "/Game/Assets/Blueprints/Iencli/BP_CharaClient.BP_CharaClient_C" (Math|Transform|MakeTransform (Transformation|GetActorLocation (Variables|Default|GetSpawnClientPoint)) "0, 0, 0" "1.000000,1.000000,1.000000") "AlwaysSpawn" "MultiplyWithRoot" 0 0))
      (Utilities|Array|Add (Variables|Default|GetClientArray) _returnvalue))
    (:then_1
      (if (== (Variables|Default|GetIndexClient) 0)
        (Default|MovetoLocation (Utilities|Array|Get(acopy) (Variables|Default|GetClientArray)) (Transformation|GetActorLocation _clientdestination) (Transformation|GetActorRotation _clientdestination))
        (Math|Integer|IncrementInt (Variables|Default|GetIndexClient)
          (:%20%20
            (CallFunction|SpawnRecette)))
        (else
          (Default|MovetoLocation (Utilities|Array|Get(acopy) _clientarray (Variables|Default|GetIndexClient)) (- (Transformation|GetActorLocation (Utilities|Array|Get(acopy) _clientarray (- (Variables|Default|GetIndexClient) 1))) "100.000000,0.000000,0.000000") "0, 0, 0")
          (Math|Integer|IncrementInt (Variables|Default|GetIndexClient)
            (:%20%20
              (CallFunction|SpawnRecette)
              (if (== (Variables|Default|GetIndexClient) (Utilities|Array|LastIndex (Variables|Default|GetClientArray)))
                (Variables|Default|SetIndexClient 0)))))))))

(event Custom|SpawnRecette
  (bind _outrownames (DataTable|GetDataTableRowNames "/Game/Assets/Blueprints/DataTable/DataRecette.DataRecette"))
  (bind _output_get (Variables|Default|SetRecetteName (.OutItem (Utilities|Array|Random _outrownames)) :!label _label))
  (bind _returnvalue (Utilities|GetDataTableRow "/Game/Assets/Blueprints/DataTable/DataRecette.DataRecette" _output_get)
    (:then
      (if (CallFunction|SelectRecette (.BubbleRequired (Utilities|Struct|BreakS_Recette _returnvalue)))
        (bind _returnvalue_2 (UserInterface|CreateWidget "/Game/Assets/UserWidget/WBP_Recette.WBP_Recette_C" 0 (.IconBubbleRequired (Utilities|Struct|BreakS_Recette _returnvalue)) (.BubbleRequired (Utilities|Struct|BreakS_Recette _returnvalue)) (.ScoreCoef (Utilities|Struct|BreakS_Recette _returnvalue)) (.Score (Utilities|Struct|BreakS_Recette _returnvalue)) (.ColorClient (Utilities|Struct|BreakS_Recette _returnvalue))))
        (Utilities|Array|Add (Variables|Default|GetRecetteWidgetArray) _returnvalue_2)
        (Class|HorizontalBox|AddChildtoHorizontalBox (Variables|/Game/Assets/UserWidget/WBP_HUD.WBP_HUD_C|GetHb_Recette (Variables|/Game/Assets/Blueprints/Game/BP_PlayerController.BP_PlayerController_C|GetHUDRef (CallFunction|GetPlayerControllerRef))) _returnvalue_2)
        (Class|Image|SetBrush (Variables|/Game/Assets/UserWidget/WBP_Recette.WBP_Recette_C|GetBubbleTeaIcon _returnvalue_2) (Utilities|Struct|MakeSlateBrush "Image" "NoTile" "NoMirror" (Utilities|Struct|MakeDeprecateSlateVector2D 75.0 104.166667) "(Left=0.000000,Top=0.000000,Right=0.000000,Bottom=0.000000)" "(SpecifiedColor=(R=1.000000,G=1.000000,B=1.000000,A=1.000000),ColorUseRule=UseColor_Specified)" "(CornerRadii=(X=0.000000,Y=0.000000,Z=0.000000,W=0.000000),Color=(SpecifiedColor=(R=0.000000,G=0.000000,B=0.000000,A=0.000000),ColorUseRule=UseColor_Specified),Width=0.000000,RoundingType=HalfHeightRadius,bUseBrushTransparency=False)" (.SpriteBubbleTea (Utilities|Struct|BreakS_Recette _returnvalue))))
        (Default|SetUpIconRequired _returnvalue_2)
        (CallFunction|SpawnerRecette)
        (else
          (goto _label))))))

(event EventBeginPlay
  ;[1 1 1] Timer Spawn Management
  (CallFunction|FirstBubbleTeaSpawn)
  (switch Utilities|FlowControl|Switch|SwitchonEnum_Difficulty (Variables|Default|GetDifficultyEnum)
    (:NewEnumerator0
      (Variables|Default|SetSpawnRecetteMinRate 17.0)
      (Variables|Default|SetSpawnRecetteMaxRate 22.0))
    (:NewEnumerator1
      (Variables|Default|SetSpawnRecetteMinRate 13.0)
      (Variables|Default|SetSpawnRecetteMaxRate 17.0))
    (:NewEnumerator2
      (Variables|Default|SetSpawnRecetteMinRate 1e+01)
      (Variables|Default|SetSpawnRecetteMaxRate 14.0))))

(fn ConstructionScript)

(fn SelectRecette
  (params (RequiredBubbleArray :type Array%20of%20Enum_BubbleType%20Enums :default "NewEnumerator0"))
  (bind _returnvalue (Utilities|Array|LastIndex RequiredBubbleArray))
  (switch Utilities|FlowControl|Switch|SwitchonEnum_Difficulty (Variables|Default|GetDifficultyEnum)
    (:NewEnumerator0
      (Variables|Default|SetChanceRate (select (== _returnvalue 0) 0.6 (select (== _returnvalue 1) 0.3 0.1))))
    (:NewEnumerator1
      (Variables|Default|SetChanceRate (select (== _returnvalue 0) 0.4 (select (== _returnvalue 1) 0.4 0.2))))
    (:NewEnumerator2
      (Variables|Default|SetChanceRate (select (== _returnvalue 0) 0.35 (select (== _returnvalue 1) 0.35 0.3)))))
  (return (> (Variables|Default|GetChanceRate) (Math|Random|RandomFloatinRange 0.0 1.0))))