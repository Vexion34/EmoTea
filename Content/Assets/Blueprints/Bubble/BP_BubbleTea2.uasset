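; Bubble tea actor that the player can pick up through an Interaction event.
; On pickup, if the player's held-item state allows it, it registers itself as the held item and snaps to the player's GrabbingScene.
; It then disables its cylinder collision and removes itself from the spawn manager's BubbleTeaArray.
; On BeginPlay it caches a reference to its WBP_IconRecette recipe icon widget.
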(event Custom|TakeBubbleTea
  (params (PlayerRef :type BP%20Player%20Object%20Reference))
  (if (Utilities|Enum|Equal(Enum) (Variables|/Game/Assets/Blueprints/Player/BP_Player.BP_Player_C|GetItemHeld PlayerRef) "NewEnumerator0")
    (Variables|/Game/Assets/Blueprints/Player/BP_Player.BP_Player_C|SetItemHeld PlayerRef "NewEnumerator6")
    (Variables|/Game/Assets/Blueprints/Player/BP_Player.BP_Player_C|SetItemRef PlayerRef self)
    (Transformation|AttachComponentToComponent self (Variables|/Game/Assets/Blueprints/Player/BP_Player.BP_Player_C|GetGrabbingScene PlayerRef) "None" "SnapToTarget" "SnapToTarget" "KeepWorld" true)
    (Collision|SetCollisionEnabled (Variables|Default|GetCylinder) "NoCollision")
    (Utilities|Array|RemoveItem (Variables|/Game/Assets/Blueprints/Bubble/BP_SpawnerManager.BP_SpawnerManager_C|GetBubbleTeaArray (CallFunction|GetSpawnManager)) self)))

(event EventBeginPlay
  (bind _aswbp_icon_recette (Utilities|Casting|CastToWBP_IconRecette (UserInterface|GetUserWidgetObject (Variables|Default|GetWidget))))
  (Variables|Default|SetIconRecetteRef _aswbp_icon_recette))

(event Collision|EventActorBeginOverlap
  (params (OtherActor :type Actor%20Object%20Reference)))

(event EventInteraction
  (params (PlayerRef :type BP%20Player%20Object%20Reference))
  (CallFunction|TakeBubbleTea PlayerRef))

(fn ConstructionScript)