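; BP_BubbleLove is a love bubble actor that descends from its placed or spawned position to hover just above the surface below.
; On BeginPlay it gives three Niagara trails random vertical speeds and traces straight down for static or dynamic world objects.
; On a hit, a timeline with an adjustable duration sweeps the actor down to that point, then resets the trail speeds when finished.
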(event EventBeginPlay
  (bind _returnvalue (Transformation|GetActorLocation))
  (|CallParentFunction)
  (bind _output_get (Variables|Default|SetNiagaraArray (Utilities|Array|MakeArray (Variables|Default|GetNS_LoveBubbleTrail) (Variables|Default|GetNS_LoveBubbleTrail1) (Variables|Default|GetNS_LoveBubbleTrail2))))
  (for _array_element _output_get
    (Niagara|SetNiagaraVariable(Vector3) _array_element "Speed" (Math|Vector|MakeVector 0.0 0.0 (Math|Random|RandomFloatinRange 25.0 3e+02))))
  (Components|Timeline|SetPlayRate (Variables|Default|GetFallDownTimeline) (/ 1.0 (Variables|Default|GetTimelineRate)))
  (bind (_outhit _returnvalue_2) (Collision|LineTraceForObjects _returnvalue (- _returnvalue "0.000000,0.000000,10000.000000") (Utilities|Array|MakeArray "ObjectTypeQuery1" "ObjectTypeQuery2") false 0 "None"))
  (if _returnvalue_2
    (Variables|Default|SetLocation (+ (.Location (Collision|BreakHitResult _outhit)) "0.000000,0.000000,80.000000"))
    (Variables|Default|SetStartLocation (Transformation|GetActorLocation))
    (bind _falltrack (Timeline|FallDownTimeline Play)
      (:Update
        (Transformation|SetActorLocation (Math|Vector|Lerp(Vector) (Variables|Default|GetStartLocation) (Variables|Default|GetLocation) _falltrack) true false))
      (:Finished
        (for _array_element_2 (Variables|Default|GetNiagaraArray)
          (Niagara|SetNiagaraVariable(Vector3) _array_element_2 "Speed" (Math|Vector|MakeVector 0.0 0.0 0.0)))))))

(fn ConstructionScript
  (|CallParentFunction))