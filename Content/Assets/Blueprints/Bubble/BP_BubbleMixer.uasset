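; BP_BubbleMixer is an interactable blender station that turns bubbles carried by the player into a bubble tea.
; It stores up to three distinct bubble types with widget icons, then consumes a held cup to start a timer-driven progress bar.
; When finished, an empty-handed interaction spawns a filled BP_BubbleTea2, using an order-independent DataTable recipe match for materials and icon.
; It also toggles a custom-depth stencil outline.
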(event Custom|TimerPreparation
  (Widget|SetVisibility (Variables|/Game/Assets/UserWidget/MixerHUD/WBP_IconContainer.WBP_IconContainer_C|GetPb_Time (Variables|Default|GetWidgetContainer)) "Visible")
  (Variables|Default|SetInPreparation true)
  (bind _returnvalue (Utilities|Time|SetTimerbyEvent (delegate Custom|LaunchTimer) 0.1 true))
  (Variables|Default|SetTimerRef _returnvalue)
  (Audio|PlaySoundatLocation "/Game/Assets/SFX/SFX_Blender.SFX_Blender" (Transformation|GetActorLocation) "0, 0, 0" 1.0 1.0 0.0 0 0 0 0))

(event Custom|LaunchTimer
  (bind _widgetcontainer (Variables|Default|GetWidgetContainer))
  (bind _widgetcontainer_2 (Variables|Default|GetWidgetContainer))
  (bind _output_get (Variables|/Game/Assets/UserWidget/MixerHUD/WBP_IconContainer.WBP_IconContainer_C|SetTimeValue _widgetcontainer (Math|Float|Clamp(Float) (+ (Variables|/Game/Assets/UserWidget/MixerHUD/WBP_IconContainer.WBP_IconContainer_C|GetTimeValue _widgetcontainer) 0.025))))
  (if (== _output_get 1.0)
    (Utilities|Time|ClearandInvalidateTimerbyHandle (Variables|Default|GetTimerRef))
    (Variables|/Game/Assets/UserWidget/MixerHUD/WBP_IconContainer.WBP_IconContainer_C|SetTimeValue (Variables|Default|GetWidgetContainer) 0.0)
    (Default|FinishIcon _widgetcontainer_2)
    (Widget|SetVisibility (Variables|/Game/Assets/UserWidget/MixerHUD/WBP_IconContainer.WBP_IconContainer_C|GetPb_Time _widgetcontainer_2) "Hidden")
    (Variables|Default|SetCanTakeBubbleTea true)
    (Audio|PlaySound2D "/Game/Assets/SFX/Blender/SC_BlenderFinished.SC_BlenderFinished" 1.0 1.0 0.0 0 0)))

(event Custom|SpawnBubbleTea
  (params (PlayerRef :type BP%20Player%20Object%20Reference))
  (bind _bubblearraytype (Variables|Default|GetBubbleArrayType))
  (bind _returnvalue (Game|SpawnActorfromClass "/Game/Assets/Blueprints/Bubble/BP_BubbleTea2.BP_BubbleTea2_C" (Math|Transform|MakeTransform "0, 0, 0" "0, 0, 0" "1.000000,1.000000,1.000000") "AlwaysSpawn" "MultiplyWithRoot" 0 0))
  (Default|TakeBubbleTea _returnvalue PlayerRef)
  (Components|StaticMesh|SetStaticMesh (Variables|/Game/Assets/Blueprints/Bubble/BP_BubbleTea2.BP_BubbleTea2_C|GetCylinder _returnvalue) "/Game/Assets/Meshes/SM_BubbleTea_Plein.SM_BubbleTea_Plein")
  (CallFunction|FindRecette)
  (Rendering|Material|SetMaterial (Variables|/Game/Assets/Blueprints/Bubble/BP_BubbleTea2.BP_BubbleTea2_C|GetCylinder _returnvalue) 3 (Variables|Default|GetBubble%20Color%20in%20Bubble%20Tea%201))
  (Rendering|Material|SetMaterial (Variables|/Game/Assets/Blueprints/Bubble/BP_BubbleTea2.BP_BubbleTea2_C|GetCylinder _returnvalue) 4 (Variables|Default|GetBubble%20Color%20in%20Bubble%20Tea%202))
  (Default|SetRecetteIcon (Variables|/Game/Assets/Blueprints/Bubble/BP_BubbleTea2.BP_BubbleTea2_C|GetIconRecetteRef _returnvalue) (Variables|Default|GetRecetteSprite))
  (Variables|/Game/Assets/Blueprints/Bubble/BP_BubbleTea2.BP_BubbleTea2_C|SetArrayTypeBubble _returnvalue _bubblearraytype)
  (Utilities|Array|Clear _bubblearraytype))

(event Custom|FindRecette
  (bind _outrownames (DataTable|GetDataTableRowNames (Variables|Default|GetDataTableRecette)))
  (bind _array_element (Utilities|Array|ForEachLoopwithBreak _outrownames :!label _label)
    (:LoopBody
      (bind _returnvalue (Utilities|GetDataTableRow (Variables|Default|GetDataTableRecette) _array_element)
        (:then
          (if (== (Utilities|Array|LastIndex (Variables|Default|GetBubbleArrayType)) (Utilities|Array|LastIndex (.BubbleRequired (Utilities|Struct|BreakS_Recette _returnvalue))))
            (for _array_element_2 (.BubbleRequired (Utilities|Struct|BreakS_Recette _returnvalue))
              (if (!= (Utilities|Array|FindItem (Variables|Default|GetBubbleArrayType) _array_element_2) -1)
                (Math|Integer|IncrementInt (Variables|Default|GetFindCount)
                  (:%20%20
                    (if (== (Variables|Default|GetFindCount) (Utilities|Array|Length (.BubbleRequired (Utilities|Struct|BreakS_Recette _returnvalue))))
                      (bind _output_get (Variables|Default|SetRecetteName _array_element))
                      (Development|PrintString (Utilities|String|ToString(Name) _output_get) true true "(R=0.000000,G=0.213542,B=0.087491,A=1.000000)" 8.0)
                      (Variables|Default|SetRecetteSprite (.SpriteBubbleTea (Utilities|Struct|BreakS_Recette _returnvalue)))
                      (Variables|Default|SetBubble%20Color%20in%20Bubble%20Tea%201 (.BubbleColorInBubbleTea1 (Utilities|Struct|BreakS_Recette _returnvalue)))
                      (Variables|Default|SetBubble%20Color%20in%20Bubble%20Tea%202 (.BubbleColorInBubbleTea2 (Utilities|Struct|BreakS_Recette _returnvalue)))
                      (goto _label Break))))))
            (Variables|Default|SetFindCount 0)))))))

(event EventManageOutline
  (params (Active? :type Boolean))
  (Rendering|SetCustomDepthStencilValue (Variables|Default|GetCylinder) (Math|Integer|SelectInt 2 1 Active?)))

(event Collision|EventActorBeginOverlap
  (params (OtherActor :type Actor%20Object%20Reference)))

(event EventBeginPlay
  (bind _returnvalue (Actor|GetActorOfClass "/Script/ColorCorrectRegions.ColorCorrectionRegion"))
  (Utilities|Set|Add (Variables|/Script/ColorCorrectRegions.ColorCorrectRegion|GetAffectedActors _returnvalue) (Utilities|ResolveSoftReference self))
  (bind _aswbp_icon_container (Utilities|Casting|CastToWBP_IconContainer (UserInterface|GetUserWidgetObject (Variables|Default|GetWidget))))
  (Variables|Default|SetWidgetContainer _aswbp_icon_container))

(event EventInteraction
  (params (PlayerRef :type BP%20Player%20Object%20Reference))
  (bind _bubblearraytype (Variables|Default|GetBubbleArrayType))
  (if (not (Variables|Default|GetInPreparation))
    (bind _itemref (Variables|/Game/Assets/Blueprints/Player/BP_Player.BP_Player_C|GetItemRef PlayerRef)
      (:then
        (bind _asbp_bubble_parents (Utilities|Casting|CastToBP_BubbleParents _itemref)
          (:then
            (Audio|PlaySound2D "/Game/Assets/SFX/PickUp/SC_PickupBubble.SC_PickupBubble" 1.0 1.0 0.0 0 0)
            (Default|DeactivateNiagaraBubble PlayerRef)
            (if (< (Utilities|Array|LastIndex _bubblearraytype) 2)
              (if (not (Utilities|Array|ContainsItem _bubblearraytype (Variables|/Game/Assets/Blueprints/Bubble/BP_BubbleParents.BP_BubbleParents_C|GetEnumBubble _asbp_bubble_parents)))
                (Utilities|Array|Add (Variables|Default|GetBubbleArrayType) (Variables|/Game/Assets/Blueprints/Bubble/BP_BubbleParents.BP_BubbleParents_C|GetEnumBubble _asbp_bubble_parents))
                (Default|SetUpIconContainer (Variables|Default|GetWidgetContainer) (Variables|/Game/Assets/Blueprints/Bubble/BP_BubbleParents.BP_BubbleParents_C|GetIconBubble _asbp_bubble_parents))
                (Actor|DestroyActor _asbp_bubble_parents)
                (Default|BreakEffect PlayerRef)
                (Variables|/Game/Assets/Blueprints/Player/BP_Player.BP_Player_C|SetItemHeld PlayerRef "NewEnumerator0"))))
          (:CastFailed
            (if (Utilities|Array|IsNotEmpty (Variables|Default|GetBubbleArrayType))
              (bind _asbp_bubble_tea_2 (Utilities|Casting|CastToBP_BubbleTea2 _itemref))
              (CallFunction|TimerPreparation)
              (Variables|/Game/Assets/Blueprints/Player/BP_Player.BP_Player_C|SetItemHeld PlayerRef "NewEnumerator0")
              (Actor|DestroyActor _asbp_bubble_tea_2)))))
      (:else))
    (elif (Variables|Default|GetCanTakeBubbleTea)
      (Variables|/Game/Assets/Blueprints/Player/BP_Player.BP_Player_C|GetItemRef PlayerRef
        (:then)
        (:else
          (CallFunction|SpawnBubbleTea PlayerRef)
          (Variables|Default|SetCanTakeBubbleTea false)
          (Variables|Default|SetInPreparation false)
          (Default|ReverseFinishIcon (Variables|Default|GetWidgetContainer))
          (Development|PrintString "Hello" true true "(R=0.842601,G=0.000000,B=1.000000,A=1.000000)" 4.0))))))

(fn ConstructionScript)