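; BP_BubbleParents is an emotion bubble pickup, apparently a parent class, that the player grabs when their item slot is at its default.
; Interaction maps the bubble's emotion to the player's held item, attaches it to GrabbingScene, disables collision, plays sound and rumble, and triggers the matching player effect.
; On BeginPlay it registers with the level's ColorCorrectionRegion.
; Other events toggle collision and switch the sphere's custom depth stencil for outlining.
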(event EventManageOutline
  (params (Active? :type Boolean))
  (Rendering|SetCustomDepthStencilValue (Variables|Default|GetSphere) (Math|Integer|SelectInt 2 1 Active?)))

(event EventManageCollisions
  (params (CollisionsOFF? :type Boolean))
  (Collision|SetCollisionEnabled (Variables|Default|GetSphere) (select CollisionsOFF? "NoCollision" "QueryAndPhysics")))

(event EventInteraction
  (params (PlayerRef :type BP%20Player%20Object%20Reference))
  (if (Utilities|Enum|Equal(Enum) (Variables|/Game/Assets/Blueprints/Player/BP_Player.BP_Player_C|GetItemHeld PlayerRef) "NewEnumerator0")
    (Variables|/Game/Assets/Blueprints/Player/BP_Player.BP_Player_C|SetItemHeld PlayerRef (Utilities|Select :Index (Variables|Default|GetEnumBubble) :NewEnumerator0 "NewEnumerator3" :NewEnumerator1 "NewEnumerator2" :NewEnumerator2 "NewEnumerator3" :NewEnumerator3 "NewEnumerator4"))
    (Variables|/Game/Assets/Blueprints/Player/BP_Player.BP_Player_C|SetItemRef PlayerRef self)
    (Transformation|AttachComponentToComponent self (Variables|/Game/Assets/Blueprints/Player/BP_Player.BP_Player_C|GetGrabbingScene PlayerRef) "None" "SnapToTarget" "SnapToTarget" "KeepWorld" true)
    (Collision|SetCollisionEnabled (Variables|Default|GetSphere) "NoCollision")
    (Audio|PlaySound2D "/Game/Assets/SFX/PickUp/SC_PickupBubble.SC_PickupBubble" 1.0 1.0 0.0 0 0)
    (Game|Feedback|PlayDynamicForceFeedback (Game|GetPlayerController 0) 0.2 0.1 true true true true)
    (switch Utilities|FlowControl|Switch|SwitchonEnum_BubbleType (Variables|Default|GetEnumBubble)
      (:NewEnumerator1
        (Default|LoveEffect PlayerRef))
      (:NewEnumerator2
        (Default|JoyEffect PlayerRef))
      (:NewEnumerator3
        (Default|AngryEffect PlayerRef)))))

(event EventBeginPlay
  (bind _returnvalue (Actor|GetActorOfClass "/Script/ColorCorrectRegions.ColorCorrectionRegion"))
  (Utilities|Set|Add (Variables|/Script/ColorCorrectRegions.ColorCorrectRegion|GetAffectedActors _returnvalue) (Utilities|ResolveSoftReference self)))

(fn ConstructionScript)